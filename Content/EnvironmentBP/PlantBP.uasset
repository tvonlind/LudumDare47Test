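; PlantBP is a waterable plant that grows as water droplets land on it and reports to the GameManager once fully watered.
; Each WaterDroplets_BP overlap with WateringRadius increments CurrentWater.
; Below MaxWater, the hit stretches PlantTrunk's Z scale by a small compounding factor.
; At MaxWater or above, it sets HasWateredPlant on GameManager instead, with debug prints along the way.
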(event OnComponentBeginOverlap(WateringRadius)
  (params (OverlappedComponent :type Primitive%20Component%20Object%20Reference) (OtherActor :type Actor%20Object%20Reference) (OtherComp :type Primitive%20Component%20Object%20Reference) (OtherBodyIndex :type Integer) (bFromSweep :type Boolean) (SweepResult :type Hit%20Result%20Structure%20%28by%20ref%29))
  (bind _currentwater (Variables|Default|GetCurrentWater))
  (bind _planttrunk (Variables|Default|GetPlantTrunk))
  (bind _returnvalue (Transformation|GetWorldScale _planttrunk))
  (Development|PrintString "Plant is hit")
  (if (== (Utilities|GetClass OtherActor) "/Game/EnvironmentBP/WateringCan/WaterDroplets_BP.WaterDroplets_BP_C")
    (Math|Float|IncrementFloat _currentwater
      (:%20%20
        (if (>= _currentwater (Variables|Default|GetMaxWater))
          (Variables|/Game/GameManagerBP.GameManagerBP_C|SetHasWateredPlant (Variables|Default|GetGameManager) true)
          (Development|PrintString "Plant has been watered")
          (else
            ;[1 1 1] Grow the plant when it has been watered
            (Transformation|SetWorldScale3D _planttrunk (Math|Vector|MakeVector (.x _returnvalue) (.y _returnvalue) (* (.z _returnvalue) 1.01)))))))))

(event EventBeginPlay)

(event Collision|EventActorBeginOverlap
  (params (OtherActor :type Actor%20Object%20Reference)))

(event EventTick
  (params (DeltaSeconds :type Float%20%28single-precision%29)))

(fn ConstructionScript)