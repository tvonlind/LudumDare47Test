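; Watering can actor that pours water when tilted and shows a text label when something is nearby.
; While body roll is within the watering angle range, Tick spawns a WaterDroplets_BP at the Sphere each frame, activates the Sprinkler and fades in the watering sound.
; Outside that range it deactivates the Sprinkler and fades the sound out.
; Sphere1 overlaps toggle WaterText, which turns to face the player pawn every tick.
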(event OnComponentBeginOverlap(Sphere1)
  (params (OverlappedComponent :type Primitive%20Component%20Object%20Reference) (OtherActor :type Actor%20Object%20Reference) (OtherComp :type Primitive%20Component%20Object%20Reference) (OtherBodyIndex :type Integer) (bFromSweep :type Boolean) (SweepResult :type Hit%20Result%20Structure%20%28by%20ref%29))
  (Rendering|SetVisibility (Variables|Default|GetWaterText) true false))

(event OnComponentEndOverlap(Sphere1)
  (params (OverlappedComponent :type Primitive%20Component%20Object%20Reference) (OtherActor :type Actor%20Object%20Reference) (OtherComp :type Primitive%20Component%20Object%20Reference) (OtherBodyIndex :type Integer))
  (Rendering|SetVisibility (Variables|Default|GetWaterText) false false))

(event EventBeginPlay
  (Rendering|SetVisibility (Variables|Default|GetWaterText) false false))

(event Collision|EventActorBeginOverlap
  (params (OtherActor :type Actor%20Object%20Reference)))

(event EventTick
  (params (DeltaSeconds :type Float%20%28single-precision%29))
  (bind _wateringcanbody (Variables|Default|GetWateringCanBody))
  (bind _watertext (Variables|Default|GetWaterText))
  (bind _returnvalue (Transformation|GetWorldRotation _wateringcanbody))
  (Transformation|SetWorldRotation _watertext (Math|Rotator|FindLookatRotation (Transformation|GetWorldLocation _watertext) (Transformation|GetActorLocation (Game|Player|GetPlayerPawn 0))) false false)
  (if (and (<= (.roll _returnvalue) (Variables|Default|GetMinWateringAngle)) (>= (.roll _returnvalue) (Variables|Default|GetMaxWateringAngle)))
    (Game|SpawnActorfromClass "/Game/EnvironmentBP/WateringCan/WaterDroplets_BP.WaterDroplets_BP_C" (Transformation|GetWorldTransform (Variables|Default|GetSphere)) "AdjustIfPossibleButDontSpawnIfColliding" 0 0)
    (Components|Activation|SetActive (Variables|Default|GetSprinkler) true false)
    (if (not (Audio|Components|Audio|IsPlaying (Variables|Default|GetSFX_Action_UsingWateringCan_Cue)))
      (Audio|Components|Audio|FadeIn (Variables|Default|GetSFX_Action_UsingWateringCan_Cue) 0.5 1.0 0.0 "Linear" :!class /Script/Engine.AudioComponent))
    (else
      (Components|Activation|SetActive (Variables|Default|GetSprinkler) false false)
      (Audio|Components|Audio|FadeOut (Variables|Default|GetSFX_Action_UsingWateringCan_Cue) 0.5 0.0 "Sin" :!class /Script/Engine.AudioComponent))))

(fn ConstructionScript)