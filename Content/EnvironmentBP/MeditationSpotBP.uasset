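; Window meditation spot where the player holds and releases left mouse to breathe, usable once per loop.
; Two overlap volumes gate it: window range enables input and shows player-facing text, while the view box shows the breath bar.
; Tick uses a gate to track hold time, count full breaths and drain the bar on release.
; Clicking locks look and movement until a click after the final breath restores control and reports "Meditate" to PauseMenu.
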(event OnComponentBeginOverlap(InWindowRange)
  (params (OverlappedComponent :type Primitive%20Component%20Object%20Reference) (OtherActor :type Actor%20Object%20Reference) (OtherComp :type Primitive%20Component%20Object%20Reference) (OtherBodyIndex :type Integer) (bFromSweep :type Boolean) (SweepResult :type Hit%20Result%20Structure%20%28by%20ref%29))
  (bind _returnvalue (Game|GetPlayerController 0))
  ;[1 1 1] Don't start checking for input unless player is near the window
  (Variables|Default|SetIsAtWindow true)
  (Input|EnableInput _returnvalue)
  (Variables|/Script/Engine.PlayerController|SetbEnableMouseOverEvents _returnvalue true)
  (Rendering|SetVisibility (Variables|Default|GetMeditationText) true false))

(event OnComponentEndOverlap(InWindowRange)
  (params (OverlappedComponent :type Primitive%20Component%20Object%20Reference) (OtherActor :type Actor%20Object%20Reference) (OtherComp :type Primitive%20Component%20Object%20Reference) (OtherBodyIndex :type Integer))
  (bind _returnvalue (Game|GetPlayerController 0))
  ;[1 1 1] Don't start checking for input unless player is near the window
  (Variables|Default|SetIsAtWindow false)
  (Input|DisableInput _returnvalue)
  (Variables|/Script/Engine.PlayerController|SetbEnableMouseOverEvents _returnvalue false)
  (Rendering|SetVisibility (Variables|Default|GetMeditationText) false false))

(event OnComponentBeginOverlap(ViewBox)
  (params (OverlappedComponent :type Primitive%20Component%20Object%20Reference) (OtherActor :type Actor%20Object%20Reference) (OtherComp :type Primitive%20Component%20Object%20Reference) (OtherBodyIndex :type Integer) (bFromSweep :type Boolean) (SweepResult :type Hit%20Result%20Structure%20%28by%20ref%29))
  ;[1 1 1] Check to see if sphere component of player is overlapping with viewbox of window
  (Variables|Default|SetIsLookingOutWindow true)
  (if (not (Variables|/Game/GameManagerBP.GameManagerBP_C|GetHasMeditated (Variables|Default|GetGameManager)))
    (Rendering|SetVisibility (Variables|Default|GetWidget) true false)))

(event OnComponentEndOverlap(ViewBox)
  (params (OverlappedComponent :type Primitive%20Component%20Object%20Reference) (OtherActor :type Actor%20Object%20Reference) (OtherComp :type Primitive%20Component%20Object%20Reference) (OtherBodyIndex :type Integer))
  ;[1 1 1] Check to see if sphere component of player is overlapping with viewbox of window
  (Variables|Default|SetIsLookingOutWindow false)
  (Rendering|SetVisibility (Variables|Default|GetWidget) false false))

(event EventBeginPlay
  (Rendering|SetVisibility (Variables|Default|GetMeditationText) false false))

(event EventTick
  (params (DeltaSeconds :type Float%20%28single-precision%29))
  (bind _meditationtext (Variables|Default|GetMeditationText))
  ;[1 1 1] Fancy solution for trying to track how long player has pressed for any given time
  (Transformation|SetWorldRotation _meditationtext (Math|Rotator|FindLookatRotation (Transformation|GetWorldLocation _meditationtext) (Transformation|GetActorLocation (Game|Player|GetPlayerPawn 0))) false false)
  (Variables|Default|SetDeltaTime DeltaSeconds)
  (bind _asbreath_bar_widget (Utilities|Casting|CastToBreathBar_Widget (UserInterface|GetUserWidgetObject (Variables|Default|GetWidget))))
  (Variables|/Game/UI/BreathBar_Widget.BreathBar_Widget_C|SetBreathProgressPercent _asbreath_bar_widget (/ (Variables|Default|GetCurrentBreathTime) (Variables|Default|GetMax%20Time%20Per%20Breath)))
  (if (Math|Boolean|ANDBoolean (Variables|Default|GetIsAtWindow) (Variables|Default|GetIsLookingOutWindow) (Game|Player|WasInputKeyJustPressed (Game|GetPlayerController 0) (Variables|Default|GetInputKey)) (not (Variables|/Game/GameManagerBP.GameManagerBP_C|GetHasMeditated (Variables|Default|GetGameManager))))
    (goto _label Open)
    (elif (Variables|Default|GetIs%20Breathing%20Out)
      ;;[1 1 1] Decrement the time holding your breath
      (if (>= (Variables|Default|GetCurrentBreathTime) 0.001)
        (bind _output_get (Variables|Default|SetCurrentBreathTime (- (Variables|Default|GetCurrentBreathTime) (Variables|Default|GetDeltaTime))))
        (Development|PrintString (Utilities|String|ToString(Float) _output_get))
        (goto _label Close)
        (else
          (Variables|Default|SetHas%20Reached%20Max%20Breath false)
          (Variables|Default|SetIs%20Breathing%20Out false)
          (goto _label Close)))
      (else
        (Utilities|FlowControl|Gate true :!label _label
          (:Exit
            (if (< (Variables|Default|GetCurrentBreathTime) (Variables|Default|GetMax%20Time%20Per%20Breath))
              (if (not (Variables|Default|GetHas%20Reached%20Max%20Breath))
                (bind _output_get_2 (Variables|Default|SetCurrentBreathTime (Class|PlayerController|GetInputKeyTimeDown (Game|GetPlayerController 0) (Variables|Default|GetInputKey))))
                (Development|PrintString (Utilities|String|ToString(Float) _output_get_2)))
              (elif (not (Variables|Default|GetHas%20Reached%20Max%20Breath))
                (Variables|Default|SetHas%20Reached%20Max%20Breath true)
                (bind _result (Math|Integer|IncrementInt (Variables|Default|GetCurrentBreaths))
                  (:%20%20
                    (Development|PrintString (Utilities|String|Append "Current breaths is " (Utilities|String|ToString(Integer) _result)))))))))))))

(event Input|MouseEvents|LeftMouseButton
  (params (Key :type Key%20Structure :default "None"))
  (bind _returnvalue (Game|GetPlayerController 0))
  (bind _returnvalue_2 (Game|GetPlayerController 0))
  (:Pressed
    (Variables|Default|SetIs%20Breathing%20Out false)
    (Variables|Default|SetInputKey Key)
    ;[1 1 1] Stop the player from moving/looking around once they start meditating
    (if (Math|Boolean|ANDBoolean (Variables|Default|GetIsLookingOutWindow) (Variables|Default|GetIsAtWindow) (not (Variables|/Game/GameManagerBP.GameManagerBP_C|GetHasMeditated (Variables|Default|GetGameManager))))
      (Input|SetIgnoreLookInput _returnvalue_2 true)
      (Input|SetIgnoreMoveInput _returnvalue_2 true)
      ;[1 1 1] Stop meditating when you've reached total breaths
      (if (< (Variables|Default|GetCurrentBreaths) (Variables|Default|GetMaxBreaths))
        (Development|PrintString "I'm meditating")
        (else
          (Development|PrintString "I'm done meditating")
          (Variables|/Game/GameManagerBP.GameManagerBP_C|SetHasMeditated (Variables|Default|GetGameManager) true)
          ;[1 1 1] Gives player back control
          (Input|ResetIgnoreLookInput _returnvalue)
          (Input|ResetIgnoreMoveInput _returnvalue)
          (Rendering|SetVisibility (Variables|Default|GetWidget) false false)
          (bind _foundwidgets (Widget|GetAllWidgetsOfClass "/Game/UI/PauseMenu.PauseMenu_C" true))
          (Default|CallActionDone (Utilities|Select :Index 0 :Option%200 _foundwidgets :Option%201 0) "Meditate")))
      (else
        (Development|PrintString "Could not meditate"))))
  (:Released
    (Variables|Default|SetIs%20Breathing%20Out true)))

(fn ConstructionScript)