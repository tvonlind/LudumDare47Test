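; Interactable journal that the player can use with a left click to mark journaling as done.
; Entering its Box enables input and shows JournalText if GameManager.HasJournaled is false; leaving disables input and hides the text.
; A click sets that flag and reports the "Journal" action to the PauseMenu widget.
; Tick keeps the text turned toward the player pawn.
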(event OnComponentBeginOverlap(Box)
  (params (OverlappedComponent :type Primitive%20Component%20Object%20Reference) (OtherActor :type Actor%20Object%20Reference) (OtherComp :type Primitive%20Component%20Object%20Reference) (OtherBodyIndex :type Integer) (bFromSweep :type Boolean) (SweepResult :type Hit%20Result%20Structure%20%28by%20ref%29))
  (Variables|Default|SetIsLookingAtJournal true)
  (if (not (Variables|/Game/GameManagerBP.GameManagerBP_C|GetHasJournaled (Variables|Default|GetGameManager)))
    (Input|EnableInput (Game|GetPlayerController 0))
    (Rendering|SetVisibility (Variables|Default|GetJournalText) true false)))

(event OnComponentEndOverlap(Box)
  (params (OverlappedComponent :type Primitive%20Component%20Object%20Reference) (OtherActor :type Actor%20Object%20Reference) (OtherComp :type Primitive%20Component%20Object%20Reference) (OtherBodyIndex :type Integer))
  (Variables|Default|SetIsLookingAtJournal false)
  (Input|DisableInput (Game|GetPlayerController 0))
  (Rendering|SetVisibility (Variables|Default|GetJournalText) false false))

(event EventBeginPlay
  (Rendering|SetVisibility (Variables|Default|GetJournalText) false false))

(event EventTick
  (params (DeltaSeconds :type Float%20%28single-precision%29))
  (bind _journaltext (Variables|Default|GetJournalText))
  (Transformation|SetWorldRotation _journaltext (Math|Rotator|FindLookatRotation (Transformation|GetWorldLocation _journaltext) (Transformation|GetActorLocation (Game|Player|GetPlayerPawn 0))) false false))

(event Input|MouseEvents|LeftMouseButton
  (params (Key :type Key%20Structure :default "None"))
  (:Pressed
    (Variables|/Game/GameManagerBP.GameManagerBP_C|SetHasJournaled (Variables|Default|GetGameManager) true)
    (bind _foundwidgets (Widget|GetAllWidgetsOfClass "/Game/UI/PauseMenu.PauseMenu_C" true))
    (Default|CallActionDone (Utilities|Select :Index 0 :Option%200 _foundwidgets :Option%201 0) "Journal")))

(fn ConstructionScript)