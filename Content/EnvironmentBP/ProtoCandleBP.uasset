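; Interactive candle that the first-person player can light or snuff with a left click while inside its trigger sphere.
; Sphere overlap toggles input and a text prompt, which turns to face the player every tick.
; Toggling switches light, flame, smoke and sound effects, updates GameManager flags and notifies the PauseMenu widget of the action.
; A looping random delay from BeginPlay varies light intensity to create flicker.
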(event OnComponentBeginOverlap(Sphere)
  (params (OverlappedComponent :type Primitive%20Component%20Object%20Reference) (OtherActor :type Actor%20Object%20Reference) (OtherComp :type Primitive%20Component%20Object%20Reference) (OtherBodyIndex :type Integer) (bFromSweep :type Boolean) (SweepResult :type Hit%20Result%20Structure%20%28by%20ref%29))
  (if (== (Utilities|GetClass OtherActor) "/Game/FirstPersonBP/Blueprints/FirstPersonCharacter.FirstPersonCharacter_C")
    (Input|EnableInput (Game|GetPlayerController 0))
    (Rendering|SetVisibility (Variables|Default|GetCandleText) true false)))

(event OnComponentEndOverlap(Sphere)
  (params (OverlappedComponent :type Primitive%20Component%20Object%20Reference) (OtherActor :type Actor%20Object%20Reference) (OtherComp :type Primitive%20Component%20Object%20Reference) (OtherBodyIndex :type Integer))
  (Input|DisableInput (Game|GetPlayerController 0))
  (Rendering|SetVisibility (Variables|Default|GetCandleText) false false))

(event EventTick
  (params (DeltaSeconds :type Float%20%28single-precision%29))
  (bind _candletext (Variables|Default|GetCandleText))
  (Transformation|SetWorldRotation _candletext (Math|Rotator|FindLookatRotation (Transformation|GetWorldLocation _candletext) (Transformation|GetActorLocation (Game|Player|GetPlayerPawn 0))) false false))

(event EventBeginPlay
  ;[1 1 1] Candle Flicker
  (Utilities|FlowControl|Delay (Math|Random|RandomFloatinRange 0.0 0.1) :!label _label)
  (Rendering|Components|Light|SetIntensity (Variables|Default|GetPointLight) (Math|Random|RandomFloatinRange 0.9 1.1))
  (goto _label))

(event Input|MouseEvents|LeftMouseButton
  (params (Key :type Key%20Structure :default "None"))
  (bind _gamemanager (Variables|Default|GetGameManager))
  (:Pressed
    (if (Variables|Default|GetIsOn)
      (Rendering|SetVisibility (Variables|Default|GetPointLight) false false)
      (Components|Activation|SetActive (Variables|Default|GetFlame) false false)
      (Rendering|SetVisibility (Variables|Default|GetFlame) false false)
      (Components|Activation|SetActive (Variables|Default|GetCandle_Smoke) true false)
      (Variables|Default|SetIsOn false)
      (Variables|/Game/GameManagerBP.GameManagerBP_C|SetHasExtinguishedCandle (Variables|Default|GetGameManager) true)
      (Audio|PlaySoundatLocation "/Game/Assets/Sound/SFX/Candle/SFX_Action_CandleSnuffed.SFX_Action_CandleSnuffed" (Transformation|GetWorldLocation (Variables|Default|GetCandle_Smoke)) "0, 0, 0" 1.0 1.0 0.0 0 0 0)
      (Development|PrintString "Candle is now off")
      (Utilities|FlowControl|Delay 0.5)
      (Components|Activation|SetActive (Variables|Default|GetCandle_Smoke) false false)
      (Components|Activation|SetActive (Variables|Default|GetBurningSFX) false false)
      (bind _foundwidgets (Widget|GetAllWidgetsOfClass "/Game/UI/PauseMenu.PauseMenu_C" true))
      (Default|CallActionDone (Utilities|Select :Index 0 :Option%200 _foundwidgets :Option%201 0) "LightOff")
      (else
        (Rendering|SetVisibility (Variables|Default|GetPointLight) true false)
        (Components|Activation|SetActive (Variables|Default|GetFlame) true false)
        (Rendering|SetVisibility (Variables|Default|GetFlame) true false)
        (Variables|Default|SetIsOn true)
        (Variables|/Game/GameManagerBP.GameManagerBP_C|SetHasLitCandle _gamemanager true)
        (Variables|/Game/GameManagerBP.GameManagerBP_C|SetHasExtinguishedCandle _gamemanager false)
        (Audio|PlaySoundatLocation "/Game/Assets/Sound/SFX/Candle/SFX_Action_CandleBeingLit.SFX_Action_CandleBeingLit" (Transformation|GetWorldLocation (Variables|Default|GetFlame)) "0, 0, 0" 1.0 1.0 0.0 0 0 0)
        (Components|Activation|SetActive (Variables|Default|GetBurningSFX) true false)
        (Development|PrintString "Candle is now on")
        (bind _foundwidgets_2 (Widget|GetAllWidgetsOfClass "/Game/UI/PauseMenu.PauseMenu_C" true))
        (Default|CallActionDone (Utilities|Select :Index 0 :Option%200 _foundwidgets_2 :Option%201 0) "LightOn")))))

(fn ConstructionScript)