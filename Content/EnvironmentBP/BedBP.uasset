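; Bed actor blueprint that lets the player end the day by clicking while standing inside its trigger box.
; Overlapping the box enables input for player controller 0 and leaving it disables input.
; A left mouse press checks GameManager.ReadyForBed, then prints a goodnight message and calls StartNewDay on the GameManager.
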(event OnComponentBeginOverlap(Box)
  (params (OverlappedComponent :type Primitive%20Component%20Object%20Reference) (OtherActor :type Actor%20Object%20Reference) (OtherComp :type Primitive%20Component%20Object%20Reference) (OtherBodyIndex :type Integer) (bFromSweep :type Boolean) (SweepResult :type Hit%20Result%20Structure%20%28by%20ref%29))
  (Input|EnableInput (Game|GetPlayerController 0)))

(event OnComponentEndOverlap(Box)
  (params (OverlappedComponent :type Primitive%20Component%20Object%20Reference) (OtherActor :type Actor%20Object%20Reference) (OtherComp :type Primitive%20Component%20Object%20Reference) (OtherBodyIndex :type Integer))
  (Input|DisableInput (Game|GetPlayerController 0)))

(event Input|MouseEvents|LeftMouseButton
  (params (Key :type Key%20Structure :default "None"))
  (:Pressed
    (if (Variables|/Game/GameManagerBP.GameManagerBP_C|GetReadyForBed (Variables|Default|GetGameManager))
      ;[1 1 1] Call function that starts fade out and resets day (Level BP?)
      (Development|PrintString "Goodnight!")
      (Default|StartNewDay (Variables|Default|GetGameManager)))))

(fn ConstructionScript)