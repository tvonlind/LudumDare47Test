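; KettleBP is a beer kit kettle that heats up while resting on a HeatingElementBP, tracking brew progress.
; Overlap events set the on-heater state and toggle the progress bar, whose widget receives the heat fraction each Tick.
; Heat rises or cools one unit per frame, independent of delta time, until full.
; Full heat latches, flags GameManager that beer is brewed and calls an empty FullyHeated effects hook.
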(event OnComponentEndOverlap(KettleBody)
  (params (OverlappedComponent :type Primitive%20Component%20Object%20Reference) (OtherActor :type Actor%20Object%20Reference) (OtherComp :type Primitive%20Component%20Object%20Reference) (OtherBodyIndex :type Integer))
  (if (== (Utilities|GetClass OtherActor) "/Game/EnvironmentBP/BeerKit/HeatingElementBP.HeatingElementBP_C")
    (Variables|Default|SetIsOnHeater false)
    (Rendering|SetVisibility (Variables|Default|GetProgressBar) false false)
    (Development|PrintString "Kettle is off heater")))

(event Custom|FullyHeated
  ;[1 1 1] Start playing boiling sounds/let off steam/rumble the pot lid?
)

(event Collision|EventActorBeginOverlap
  (params (OtherActor :type Actor%20Object%20Reference))
  (if (== (Utilities|GetClass OtherActor) "/Game/EnvironmentBP/BeerKit/HeatingElementBP.HeatingElementBP_C")
    (Variables|Default|SetIsOnHeater true)
    (Development|PrintString "Kettle is on Heater")
    (Utilities|FlowControl|Delay 0.2)
    (Rendering|SetVisibility (Variables|Default|GetProgressBar) true false)))

(event EventTick
  (params (DeltaSeconds :type Float%20%28single-precision%29))
  (bind _output_get (Variables|Default|SetPercentHeatTime (/ (Variables|Default|GetCurrentHeatTime) (Variables|Default|GetTotalHeatTime))))
  ;[1 1 1] Track time on/off heater
  (bind _asboiling_progress_bar_widget (Utilities|Casting|CastToBoilingProgressBar_Widget (UserInterface|GetUserWidgetObject (Variables|Default|GetProgressBar))))
  (Variables|/Game/UI/BoilingProgressBar_Widget.BoilingProgressBar_Widget_C|SetBoilingProgress _asboiling_progress_bar_widget _output_get)
  (if (not (Variables|Default|GetHasBeenHeated))
    (if (and (Variables|Default|GetIsOnHeater) (<= (Variables|Default|GetCurrentHeatTime) (Variables|Default|GetTotalHeatTime)))
      (Variables|Default|SetCurrentHeatTime (+ (Variables|Default|GetCurrentHeatTime) 1.0))
      (if (>= (Variables|Default|GetCurrentHeatTime) (Variables|Default|GetTotalHeatTime))
        (Variables|Default|SetHasBeenHeated true)
        (Variables|/Game/GameManagerBP.GameManagerBP_C|SetHasBrewedBeer (Variables|Default|GetGameManager) true)
        (CallFunction|FullyHeated))
      (elif (>= (Variables|Default|GetCurrentHeatTime) 1.0)
        (Variables|Default|SetCurrentHeatTime (- (Variables|Default|GetCurrentHeatTime) 1.0))))))

(fn ConstructionScript)