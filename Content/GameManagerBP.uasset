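; Game manager that tracks a daily routine of tasks (meditating, candle lighting and extinguishing, brewing, watering, journaling) and advances the day counter.
; Tick flags ReadyForBed once every task flag is set.
; StartNewDay runs a fade widget, then either resets task flags and prop progress or prints game over past MaxDays.
; Kettle and watering can return to their BeginPlay locations after a one-second delay, hiding the warp behind the fade.
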(event Custom|ResetPositionsDelay
  ;[1 1 1] Delaying for a second before reseting positions (so they don't warp until black)
  (Utilities|FlowControl|Delay 1.0)
  (CallFunction|ResetPositions))

(event EventBeginPlay
  (Variables|Default|SetCanStartingLocation (Transformation|GetActorLocation (Variables|Default|GetWateringCan)))
  (Variables|Default|SetKettleStartingLocation (Transformation|GetActorLocation (Variables|Default|GetKettle))))

(event Collision|EventActorBeginOverlap
  (params (OtherActor :type Actor%20Object%20Reference)))

(event EventTick
  (params (DeltaSeconds :type Float%20%28single-precision%29))
  ;[1 1 1] Constantly check to see if you have completed all of your tasks
  (if (and (Math|Boolean|ANDBoolean (Variables|Default|GetHasMeditated) (Variables|Default|GetHasLitCandle) (Variables|Default|GetHasBrewedBeer) (Variables|Default|GetHasWateredPlant) (Variables|Default|GetHasExtinguishedCandle) (Variables|Default|GetHasJournaled)) (not (Variables|Default|GetReadyForBed)))
    (Variables|Default|SetReadyForBed true)
    (Development|PrintString "Ready for a new day")))

(fn ConstructionScript)

(fn StartNewDay
  (bind _currentday (Variables|Default|GetCurrentDay))
  ;[1 1 1] Sets up the fade to black
  (bind _returnvalue (UserInterface|CreateWidget "/Game/UI/Fade_Widget.Fade_Widget_C" (Game|GetPlayerController 0)))
  (bind _asfade_widget (Utilities|Casting|CastToFade_Widget _returnvalue))
  (Variables|Default|SetFadeReference _asfade_widget)
  (UserInterface|Viewport|AddtoViewport _returnvalue 0)
  (Default|FadeOut (Variables|Default|GetFadeReference))
  (Math|Integer|IncrementInt _currentday
    (:%20%20
      (if (<= _currentday (Variables|Default|GetMaxDays))
        (Development|PrintString (Utilities|String|Append "This is day " (Utilities|String|ToString(Integer) (Variables|Default|GetCurrentDay))))
        (CallFunction|ResetActions)
        (CallFunction|ResetPositionsDelay)
        ;[1 1 1] Fade-in has a built in 1 second delay
        (Default|Fadein (Variables|Default|GetFadeReference))
        (else
          (Development|PrintString "Game Over!"))))))

(fn ResetActions
  (bind _kettle (Variables|Default|GetKettle))
  (Variables|Default|SetHasJournaled false)
  (Variables|Default|SetHasWateredPlant false)
  (Variables|Default|SetHasMeditated false)
  (Variables|Default|SetHasBrewedBeer false)
  (Variables|Default|SetHasLitCandle false)
  (Variables|Default|SetHasExtinguishedCandle false)
  (Variables|Default|SetReadyForBed false)
  (Variables|/Game/EnvironmentBP/MeditationSpotBP.MeditationSpotBP_C|SetCurrentBreaths (Variables|Default|GetMeditationSpot) 0)
  (Variables|/Game/EnvironmentBP/PlantBP.PlantBP_C|SetCurrentWater (Variables|Default|GetPlant) 0.0)
  (Variables|/Game/EnvironmentBP/BeerKit/KettleBP.KettleBP_C|SetCurrentHeatTime _kettle 0.0)
  (Variables|/Game/EnvironmentBP/BeerKit/KettleBP.KettleBP_C|SetHasBeenHeated _kettle false))

(fn ResetPositions
  (Transformation|SetWorldLocationAndRotation (Variables|/Game/EnvironmentBP/BeerKit/KettleBP.KettleBP_C|GetStaticMesh (Variables|Default|GetKettle)) (Variables|Default|GetKettleStartingLocation) "0, 0, 0" false false)
  (Transformation|SetWorldLocationAndRotation (Variables|/Game/EnvironmentBP/WateringCan/WateringCanBP.WateringCanBP_C|GetWateringCanBody (Variables|Default|GetWateringCan)) (Variables|Default|GetCanStartingLocation) "0, 0, 0" false false))